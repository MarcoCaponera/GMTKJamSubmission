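; BP_Platform is a possessable tilting platform for a ball-rolling game, with its own camera and chainable levels.
; Enhanced Input rotates it in pitch and roll by fixed steps, clamped to a maximum tilt.
; A reset box returns fallen balls to the start offset.
; The end trigger disables input, blends view to NextPlatform, then hands over ball and possession through Init on a timer; final platforms also show a finish widget.
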(event `self.ReceiveBeginPlay`
  (`EnhancedInputSubsystemInterface.AddMappingContext` (pcsubsystem `EnhancedInputLocalPlayerSubsystem` (`GameplayStatics.GetPlayerController` 0)) "/Game/TeamContent/Input/IMC_Platform.IMC_Platform" 0 (struct))
  (`SceneComponent.K2_SetWorldLocation` (`self.Camera`) (+ (`self.CameraOffset`) (`self.K2_GetActorLocation`)) false false)
  (set `self.Original Transform` (`self.GetTransform`)))

(event `EnhancedInput|/Game/TeamContent/Input/IA_TiltBackward`
  (params (ActionValue :type Boolean) (ElapsedSeconds :type "Float (double-precision)") (TriggeredSeconds :type "Float (double-precision)") (InputAction :type "InputAction Object Reference" :default "/Game/TeamContent/Input/IA_TiltBackward.IA_TiltBackward"))
  (bind (_returnvalue_roll _returnvalue_pitch _returnvalue_yaw) (`KismetMathLibrary.BreakRotator` (`self.K2_GetActorRotation`)))
  (bind _maxtilt (`self.MaxTilt`))
  (:`Triggered`
    (`self.K2_AddActorWorldRotation` (`KismetMathLibrary.MakeRotator` 0.0 (`self.RotSpeed`)))
    (if (>= _returnvalue_pitch _maxtilt)
      (`self.K2_SetActorRotation` (`KismetMathLibrary.MakeRotator` _returnvalue_roll _maxtilt _returnvalue_yaw)))))

(event `EnhancedInput|/Game/TeamContent/Input/IA_TiltForward`
  (params (ActionValue :type Boolean) (ElapsedSeconds :type "Float (double-precision)") (TriggeredSeconds :type "Float (double-precision)") (InputAction :type "InputAction Object Reference" :default "/Game/TeamContent/Input/IA_TiltForward.IA_TiltForward"))
  (bind (_returnvalue_roll _returnvalue_pitch _returnvalue_yaw) (`KismetMathLibrary.BreakRotator` (`self.K2_GetActorRotation`)))
  (bind _returnvalue (* (`self.MaxTilt`) -1.0))
  (:`Triggered`
    (`self.K2_AddActorWorldRotation` (`KismetMathLibrary.MakeRotator` 0.0 (* (`self.RotSpeed`) -1.0)))
    (if (<= _returnvalue_pitch _returnvalue)
      (`self.K2_SetActorRotation` (`KismetMathLibrary.MakeRotator` _returnvalue_roll _returnvalue _returnvalue_yaw)))))

(event `EnhancedInput|/Game/TeamContent/Input/IA_TiltRight`
  (params (ActionValue :type Boolean) (ElapsedSeconds :type "Float (double-precision)") (TriggeredSeconds :type "Float (double-precision)") (InputAction :type "InputAction Object Reference" :default "/Game/TeamContent/Input/IA_TiltRight.IA_TiltRight"))
  (bind (_returnvalue_roll _returnvalue_pitch _returnvalue_yaw) (`KismetMathLibrary.BreakRotator` (`self.K2_GetActorRotation`)))
  (bind _maxtilt (`self.MaxTilt`))
  (:`Triggered`
    (`self.K2_AddActorWorldRotation` (`KismetMathLibrary.MakeRotator` (`self.RotSpeed`)))
    (if (>= _returnvalue_roll _maxtilt)
      (`self.K2_SetActorRotation` (`KismetMathLibrary.MakeRotator` _maxtilt _returnvalue_pitch _returnvalue_yaw)))))

(event `EnhancedInput|/Game/TeamContent/Input/IA_TiltLeft`
  (params (ActionValue :type Boolean) (ElapsedSeconds :type "Float (double-precision)") (TriggeredSeconds :type "Float (double-precision)") (InputAction :type "InputAction Object Reference" :default "/Game/TeamContent/Input/IA_TiltLeft.IA_TiltLeft"))
  (bind (_returnvalue_roll _returnvalue_pitch _returnvalue_yaw) (`KismetMathLibrary.BreakRotator` (`self.K2_GetActorRotation`)))
  (bind _returnvalue (* (`self.MaxTilt`) -1.0))
  (:`Triggered`
    (`self.K2_AddActorWorldRotation` (`KismetMathLibrary.MakeRotator` (* (`self.RotSpeed`) -1.0)))
    (if (<= _returnvalue_roll _returnvalue)
      (`self.K2_SetActorRotation` (`KismetMathLibrary.MakeRotator` _returnvalue _returnvalue_pitch _returnvalue_yaw)))))

(event `self.ResetBox.OnComponentBeginOverlap`
  (params (OverlappedComponent :type "PrimitiveComponent Object Reference") (OtherActor :type "Actor Object Reference") (OtherComp :type "PrimitiveComponent Object Reference") (OtherBodyIndex :type Integer) (bFromSweep :type Boolean) (SweepResult :type "HitResult Structure (by ref)"))
  (`self.K2_SetActorLocation` OtherActor (+ (`self.K2_GetActorLocation`) (`self.BallStart`)) false false)
  (message `/Game/TeamContent/BP/Ball/I_Ball.f_Stop` OtherActor))

(event `self.EndOfLevelTrigger.OnComponentBeginOverlap`
  (params (OverlappedComponent :type "PrimitiveComponent Object Reference") (OtherActor :type "Actor Object Reference") (OtherComp :type "PrimitiveComponent Object Reference") (OtherBodyIndex :type Integer) (bFromSweep :type Boolean) (SweepResult :type "HitResult Structure (by ref)"))
  (bind _returnvalue (`GameplayStatics.GetPlayerController` 0))
  (bind _easetime (`self.EaseTime`))
  (`PrimitiveComponent.SetCollisionEnabled` (`self.ResetBox`) "NoCollision")
  (`self.DisableInput` _returnvalue)
  (`PlayerController.SetViewTargetWithBlend` _returnvalue (`self.NextPlatform`) _easetime "VTBlend_EaseInOut" 5.0 false)
  (`KismetSystemLibrary.K2_SetTimerDelegate` (delegate `GiveInput`) _easetime)
  (if (`self.IsFinalPlatform?`)
    (`KismetSystemLibrary.Delay` 0.5)
    (bind _returnvalue_2 (`|CreateWidget` "/Game/TeamContent/BP/Widget/WB_Finish.WB_Finish_C" (`GameplayStatics.GetPlayerController` 0)))
    (`UserWidget.AddToViewport` _returnvalue_2 0)
    (`self.K2_SetActorTransform` (`self.Original Transform`) false true)))

(event `GiveInput`
  (`self.Init` (`self.NextPlatform`) (stale `self.EndOfLevelTrigger.OnComponentBeginOverlap` OtherActor)))

(event `Init`
  (params (Ball :type "Actor Object Reference"))
  (bind _returnvalue (`GameplayStatics.GetPlayerController` 0))
  (`self.K2_SetActorLocation` Ball (+ (`self.K2_GetActorLocation`) (`self.BallStart`)) false false)
  (`PrimitiveComponent.AddImpulse` (`self.GetComponentByClass` Ball "/Script/Engine.PrimitiveComponent") (* (`self.GetVelocity` Ball) -1.0) "None" false)
  (`Controller.Possess` _returnvalue self)
  (`self.EnableInput` _returnvalue)
  (`PrimitiveComponent.SetCollisionEnabled` (`self.ResetBox`) "QueryOnly"))

(fn `UserConstructionScript`)