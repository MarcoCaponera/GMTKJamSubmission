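; BP_ShrinkObject is a trigger in the ball content that sends a shrink message to any actor overlapping it.
; When CanActivate is true, an overlap calls FShrinkMessage, plays a Niagara effect and 2D sound, then disables box collision and darkens the ReduceSize sprite.
; FReset re-arms it by restoring query-only collision and white sprite color.
; FStackcounter is a stub returning zero.
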(event `self.ReceiveActorBeginOverlap`
  (params (OtherActor :type "Actor Object Reference"))
  (if (`self.CanActivate?`)
    (message `/Game/TeamContent/BP/Ball/I_Ball.f_Shrink` OtherActor)
    (`self.Effect`)
    (`PrimitiveComponent.SetCollisionEnabled` (`self.Box`) "NoCollision")
    (`PaperFlipbookComponent.SetSpriteColor` (`self.Reduce_Size`) (struct :`A` 0.625))))

(event `Effect`
  (`NiagaraFunctionLibrary.SpawnSystemAtLocation` "/Game/TeamContent/VFX/VFX_Shrink.VFX_Shrink" (`SceneComponent.K2_GetComponentLocation` (`self.Box`)))
  (`GameplayStatics.SpawnSound2D` "/Engine/VREditor/Sounds/UI/Floating_UI_Open-002.Floating_UI_Open-002" 1.0 1.0 0.0 null))

(event `/Game/TeamContent/BP/Platform/I_Resetable.f_Reset`
  (`PrimitiveComponent.SetCollisionEnabled` (`self.Box`) "QueryOnly")
  (`PaperFlipbookComponent.SetSpriteColor` (`self.Reduce_Size`) (struct :`R` 1.0 :`G` 1.0 :`B` 1.0 :`A` 1.0)))

(fn `f_Stackcounter`
  (returns (Stacks :type Integer))
  (return 0))

(fn `UserConstructionScript`)