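; Ball actor that can grow, shrink, stop and reset in response to events, and opens the pause widget on Escape.
; Enlarge and shrink step the Sphere's world scale up to set limits, each decrementing the opposite counter, while enlarge also messages Platform for camera shake.
; Stop applies an impulse opposite to current velocity.
; Reset restores the scale saved at BeginPlay, and both shrink and reset send the shrink count to the HUD.
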(event `self.ReceiveBeginPlay`
  (bind (_returnvalue_location _returnvalue_rotation _returnvalue_scale) (`KismetMathLibrary.BreakTransform` (`SceneComponent.GetRelativeTransform` (`self.Sphere`))))
  (set `self.InitialScale` _returnvalue_scale))

(event `Key|Escape`
  (params (Key :type "Key Structure"))
  (:`Pressed`
    (bind _returnvalue (`|CreateWidget` "/Game/TeamContent/BP/Widget/WB_Pause.WB_Pause_C" (`GameplayStatics.GetPlayerController` 0)))
    (`UserWidget.AddToViewport` _returnvalue 0)))

(event `/Game/TeamContent/BP/Ball/I_Ball.f_Enlarge`
  (bind _sphere (`self.Sphere`))
  (message `/Game/TeamContent/BP/Ball/I_Ball.f_CameraShake` (`self.Platform`))
  (if (not (== (`self.CurrentEnlarge`) (`self.MaxEnlarge`)))
    (bind _result (`/Engine/EditorBlueprintResources/StandardMacros.IncrementInt` (`self.CurrentEnlarge`))
      (:`  `
        (set `self.CurrentEnlarge` _result)
        (`SceneComponent.SetWorldScale3D` _sphere (+ (`SceneComponent.K2_GetComponentScale` _sphere) (`self.ScaleAdd`)))
        (`/Engine/EditorBlueprintResources/StandardMacros.DecrementInt` (`self.CurrentShrink`))))))

(event `/Game/TeamContent/BP/Ball/I_Ball.f_Stop`
  (`PrimitiveComponent.AddImpulse` (`self.Sphere`) (* (`self.GetVelocity`) -1) "None" false))

(event `/Game/TeamContent/BP/Ball/I_Ball.f_Shrink`
  (bind _sphere (`self.Sphere`))
  (if (not (== (`self.CurrentShrink`) (`self.MaxShrink`)))
    (bind _result (`/Engine/EditorBlueprintResources/StandardMacros.IncrementInt` (`self.CurrentShrink`))
      (:`  `
        (bind _output_get (set `self.CurrentShrink` _result))
        (`SceneComponent.SetWorldScale3D` _sphere (- (`SceneComponent.K2_GetComponentScale` _sphere) (`self.ScaleSub`)))
        (`/Engine/EditorBlueprintResources/StandardMacros.DecrementInt` (`self.CurrentEnlarge`)
          (:`  `
            (message `/Game/TeamContent/BP/Widget/I_HUD.f_updateScale` (`PlayerController.GetHUD` (`GameplayStatics.GetPlayerController` 0)) _output_get)))))))

(event `/Game/TeamContent/BP/Platform/I_Resetable.f_Reset`
  (`self.SetActorScale3D` (`self.InitialScale`))
  (set `self.CurrentEnlarge` 0)
  (bind _output_get (set `self.CurrentShrink` 0))
  (message `/Game/TeamContent/BP/Widget/I_HUD.f_updateScale` (`PlayerController.GetHUD` (`GameplayStatics.GetPlayerController` 0)) _output_get))

(fn `f_Stackcounter`
  (returns (Stacks :type Integer))
  (return 0))

(fn `UserConstructionScript`)