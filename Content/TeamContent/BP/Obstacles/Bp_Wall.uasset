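; Bp_Wall is an obstacle wall that gives impact feedback when something hits its Cube component.
; On hit, it spawns a collision Niagara effect at the impact point, oriented along the negated hit normal, and plays a 2D sound.
; A CanActivate flag with a reset timer works as a cooldown, so repeated hits do not retrigger the feedback until the timer expires.
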(event `self.Cube.OnComponentHit`
  (params (HitComponent :type "PrimitiveComponent Object Reference") (OtherActor :type "Actor Object Reference") (OtherComp :type "PrimitiveComponent Object Reference") (NormalImpulse :type "Vector Structure") (Hit :type "HitResult Structure (by ref)"))
  (if (`self.CanActivate?`)
    (`NiagaraFunctionLibrary.SpawnSystemAtLocation` "/Game/TeamContent/VFX/VFX_WallCollision.VFX_WallCollision" Hit_Location (`KismetMathLibrary.Conv_VectorToRotator` (`KismetMathLibrary.NegateVector` Hit_Normal)))
    (`GameplayStatics.SpawnSound2D` "/Engine/VREditor/Sounds/UI/Floating_Ui.Floating_Ui" 1.0 1.0 0.0 null)
    (`KismetSystemLibrary.K2_SetTimerDelegate` (delegate `Reset`) (`self.Time`))
    (set `self.CanActivate?` false)))

(event `Reset`
  (set `self.CanActivate?` true))

(fn `UserConstructionScript`)