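; BP_EnlargeSelf is an obstacle that grows when hit and knocks back whatever hit it.
; A cube hit, gated by a timed cooldown, enlarges the cube and applies an impulse to the other actor along the negated hit normal.
; Growth widens X and Y scale up to a limit, after which further hits set a fixed push force.
; Each activation spawns a collision VFX and 2D sound.
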(event `self.Cube.OnComponentHit`
  (params (HitComponent :type "PrimitiveComponent Object Reference") (OtherActor :type "Actor Object Reference") (OtherComp :type "PrimitiveComponent Object Reference") (NormalImpulse :type "Vector Structure") (Hit :type "HitResult Structure (by ref)"))
  (set `self.Hit Location` Hit_Location)
  (set `self.Hit Normal` Hit_Normal)
  (if (`self.CanActivate?`)
    (`self.Enlarge`)
    (`PrimitiveComponent.AddImpulse` (`self.GetComponentByClass` OtherActor "/Script/Engine.PrimitiveComponent") (* (* Hit_Normal (`self.Force`)) -1.0) "None" false)
    (`KismetSystemLibrary.K2_SetTimerDelegate` (delegate `Reset`) (`self.Time`))
    (set `self.CanActivate?` false)))

(event `Reset`
  (set `self.CanActivate?` true))

(event `Enlarge`
  (bind _cube (`self.Cube`))
  (if (== (`self.CurrentEnlarge`) (`self.MaxEnlarge`))
    (set `self.Force` 600.0)
    (else
      (bind _result (`/Engine/EditorBlueprintResources/StandardMacros.IncrementInt` (`self.CurrentEnlarge`))
        (:`  `
          (set `self.CurrentEnlarge` _result)
          (`SceneComponent.SetWorldScale3D` _cube (+ (`SceneComponent.K2_GetComponentScale` _cube) (1.0 1.0 0.0)))))))
  (`NiagaraFunctionLibrary.SpawnSystemAtLocation` "/Game/TeamContent/VFX/VFX_ObstacleCollision.VFX_ObstacleCollision" (`self.Hit Location`) (`KismetMathLibrary.Conv_VectorToRotator` (`KismetMathLibrary.NegateVector` (`self.Hit Normal`))))
  (`GameplayStatics.SpawnSound2D` "/Engine/VREditor/Sounds/UI/Floating_UI_Open-002.Floating_UI_Open-002" 1.0 1.0 0.0 null))

(fn `UserConstructionScript`)