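; BP_Obstacle1 is an obstacle that knocks back whatever hits its Cube.
; On a hit, it sends the FEnlargeMessage call to the other actor and applies an impulse to that actor's primitive component against the hit normal.
; It spawns collision VFX and a 2D sound, then disables itself until a timer re-arms it, acting as a cooldown.
; FStackcounter is a stub that returns zero.
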(event `self.Cube.OnComponentHit`
  (params (HitComponent :type "PrimitiveComponent Object Reference") (OtherActor :type "Actor Object Reference") (OtherComp :type "PrimitiveComponent Object Reference") (NormalImpulse :type "Vector Structure") (Hit :type "HitResult Structure (by ref)"))
  (if (`self.CanActivate?`)
    (message `/Game/TeamContent/BP/Ball/I_Ball.f_Enlarge` OtherActor)
    (`PrimitiveComponent.AddImpulse` (`self.GetComponentByClass` OtherActor "/Script/Engine.PrimitiveComponent") (* (* Hit_Normal (`self.Force`)) -1.0) "None" false)
    (`self.Effect`)
    (`KismetSystemLibrary.K2_SetTimerDelegate` (delegate `Reset`) (`self.Time`))
    (set `self.CanActivate?` false)))

(event `Reset`
  (set `self.CanActivate?` true))

(event `Effect`
  (`NiagaraFunctionLibrary.SpawnSystemAtLocation` "/Game/TeamContent/VFX/VFX_Collision.VFX_Collision" (`.Location` (`GameplayStatics.BreakHitResult` (stale `self.Cube.OnComponentHit` Hit))) (`KismetMathLibrary.Conv_VectorToRotator` (`KismetMathLibrary.NegateVector` (`.Normal` (`GameplayStatics.BreakHitResult` (stale `self.Cube.OnComponentHit` Hit))))))
  (`GameplayStatics.SpawnSound2D` "/Engine/VREditor/Sounds/UI/Floating_UI_Open-002.Floating_UI_Open-002" 1.0 1.0 0.0 null))

(fn `f_Stackcounter`
  (returns (Stacks :type Integer))
  (return 0))

(fn `UserConstructionScript`)