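; Game mode for a ball game that moves player control from one level platform to the next.
; AddLevel registers each platform and has the first player controller possess the one with index 0.
; SwapLevel increments the current level and possesses the platform whose index matches it.
; SortLevels is an unfinished nested loop that reorders nothing, so selection relies on each platform's own index rather than array order.
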(event `/Game/TeamContent/BP/Gamemode/I_Gamemode.AddLevel`
  (params (Platform :type "/Game/TeamContent/BP/Platform/BP_Platform Object Reference"))
  (`KismetArrayLibrary.Array_Add` (`self.Platforms`) Platform)
  (if (== (`/Game/TeamContent/BP/Platform/BP_Platform.PlatformIndex` Platform) 0)
    (`Controller.Possess` (`GameplayStatics.GetPlayerController` 0) Platform)
    (`KismetSystemLibrary.PrintString` (`KismetSystemLibrary.GetDisplayName` Platform))))

(event `/Game/TeamContent/BP/Gamemode/I_Gamemode.SwapLevel`
  (`/Engine/EditorBlueprintResources/StandardMacros.IncrementInt` (`self.CurrentLevel`)
    (:`  `
      (for _array_element (`self.Platforms`)
        (if (== (`/Game/TeamContent/BP/Platform/BP_Platform.PlatformIndex` _array_element) (`self.CurrentLevel`))
          (`Controller.Possess` (`GameplayStatics.GetPlayerController` 0) _array_element)
          (`KismetSystemLibrary.PrintString` "Swap"))))))

(fn `SortLevels`
  (bind _platforms (`self.Platforms`))
  (for (_ _array_index) _platforms
    (for _ (range (+ _array_index 1) (+ (`KismetArrayLibrary.Array_Length` _platforms) 1))
      _)))

(fn `UserConstructionScript`)